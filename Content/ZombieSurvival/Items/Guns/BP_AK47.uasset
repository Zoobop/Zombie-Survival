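; BP_AK47 is the AK47 gun Blueprint for the zombie survival game, handling its firing cosmetics and hit feedback.
; Gun start-fire calls StartFireMulticast, which runs the Fire Animation and Effects graph.
; That graph plays a montage on the owner's mesh, attaches the gunshot sound at the Muzzle and briefly unhides the muzzle flash.
; Entity hits only print debug details such as actor, bone, distance and damage.
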(event Custom|Start%20Fire%20Multicast
  (params (Gun%20Owner :type Entity%20Object%20Reference))
  (|FireAnimationandEffects Gun%20Owner 0.1))

(event EventOnEntityHit
  (params (GunOwner :type Entity%20Object%20Reference) (Damage :type Integer) (Hit :type Hit%20Result%20Structure))
  (Development|PrintString (Utilities|String|ToString(Text) (Utilities|Text|FormatText "{Hit Actor} - Bone: {Bone Name} - Distance Away: {Distance} - Time: {Time} - Damage Done: {Damage}" (Utilities|GetDisplayName (.hitactor Hit)) (.hitbonename Hit) (.distance Hit) (.time Hit) Damage)) true true "(R=0.000000,G=0.660000,B=1.000000,A=1.000000)" 0.5))

(event EventOnGunStartFire
  (params (GunOwner :type Entity%20Object%20Reference))
  (CallFunction|StartFireMulticast GunOwner))

(fn ConstructionScript)