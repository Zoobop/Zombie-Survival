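; BP_AR15 is the AR-15 gun Blueprint for the zombie survival game, handling the cosmetic effects of firing.
; When firing starts, it calls StartFireMulticast, which plays the fire montage on the owner's mesh.
; That event also spawns a pitch-shifted gunshot sound at the Muzzle attach point and briefly unhides the muzzle flash.
; The Blueprint itself contains no damage, ammo or projectile logic.
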(event Custom|Start%20Fire%20Multicast
  (params (Gun%20Owner :type Entity%20Object%20Reference))
  (bind _muzzleflash (Variables|Default|GetMuzzleFlash))
  (Animation|Montage|PlayMontage (Variables|/Script/Engine.Character|GetMesh Gun%20Owner) (Variables|Default|GetFireAnimation)
    (:then
      (Audio|SpawnSoundAttached "/Game/ZombieSurvival/Sounds/WAV/Gunshot_AR15.Gunshot_AR15" (Variables|Default|GetSkeletalMeshComponent) "Muzzle" "0, 0, 0" "0, 0, 0" "SnapToTarget" false 1.0 15.0 0.0 0 0)
      (Development|SetHiddeninGame _muzzleflash false false)
      (Utilities|FlowControl|Delay 0.05)
      (Development|SetHiddeninGame _muzzleflash true false))))

(event EventOnGunStartFire
  (params (GunOwner :type Entity%20Object%20Reference))
  (CallFunction|StartFireMulticast GunOwner))

(fn ConstructionScript)