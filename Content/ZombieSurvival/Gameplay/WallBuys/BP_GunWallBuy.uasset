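; Wall-mounted gun purchase for zombie survival that sells a weapon to soldiers for points, or an ammo refill if they already own it.
; Trigger overlap picks the price, shows the hold-F prompt and, on authority, registers the purchasable with the soldier.
; Activate passes through a gate opened by that overlap to call Purchase.
; First-buy and refill handlers add the gun or load bullets and deduct points, running both locally and through server events for clients.
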(event OnComponentBeginOverlap(PurchaseTrigger)
  (params (OverlappedComponent :type Primitive%20Component%20Object%20Reference) (OtherActor :type Actor%20Object%20Reference) (OtherComp :type Primitive%20Component%20Object%20Reference) (OtherBodyIndex :type Integer) (bFromSweep :type Boolean) (SweepResult :type Hit%20Result%20Structure%20%28by%20ref%29))
  (bind (_asbp_soldier _bsuccess) (Utilities|Casting|CastToBP_Soldier OtherActor))
  (if _bsuccess
    (Utilities|AdjustActionText _asbp_soldier)
    (Default|DisplayActionText _asbp_soldier (Class|PurchasableInterface|GetDisplayText))
    (Networking|SwitchHasAuthority
      (:Authority
        (Default|InteractwithPurchaseable _asbp_soldier self true)
        (Input|EnableInput (Game|GetPlayerController 0))
        (Utilities|FlowControl|Gate true) ; enters at Open
      ))))

(event OnComponentEndOverlap(PurchaseTrigger)
  (params (OverlappedComponent :type Primitive%20Component%20Object%20Reference) (OtherActor :type Actor%20Object%20Reference) (OtherComp :type Primitive%20Component%20Object%20Reference) (OtherBodyIndex :type Integer))
  (bind (_asbp_soldier _bsuccess) (Utilities|Casting|CastToBP_Soldier OtherActor))
  (if _bsuccess
    (Default|RemoveActionText _asbp_soldier)
    (Networking|SwitchHasAuthority
      (:Authority
        (Default|InteractwithPurchaseable _asbp_soldier self false)
        (Input|DisableInput (Game|GetPlayerController 0))))))

(event Custom|Server%20On%20Refill
  (params (Player :type Soldier%20Object%20Reference))
  (Utilities|HandleRefill Player))

(event Custom|Server%20On%20First%20Time%20Purchase
  (params (Player :type Soldier%20Object%20Reference))
  (Utilities|HandleFirstTimePurchase Player))

(event EventActivate
  (Utilities|FlowControl|Gate true
    (:Exit
      (Class|WallBuy|Purchase (.AsBP%20Soldier (Utilities|Casting|CastToBP_Soldier (stale OnComponentBeginOverlap(PurchaseTrigger) OtherActor))))
      (Default|RemoveActionText (.AsBP%20Soldier (Utilities|Casting|CastToBP_Soldier (stale OnComponentBeginOverlap(PurchaseTrigger) OtherActor)))))))

(event EventOnFirstTimePurchase
  (params (Player :type Soldier%20Object%20Reference))
  (if (Ability|HasAuthority Player)
    (Utilities|HandleFirstTimePurchase Player)
    (else
      (CallFunction|ServeronFirstTimePurchase Player)
      (Utilities|HandleFirstTimePurchase Player))))

(event EventOnRefill
  (params (Player :type Soldier%20Object%20Reference))
  (if (Ability|HasAuthority Player)
    (Utilities|HandleRefill Player)
    (else
      (CallFunction|ServeronRefill Player)
      (Utilities|HandleRefill Player))))

(fn ConstructionScript)

(fn GetDisplayText
  (if (== (Variables|Default|GetCost) (Variables|Default|GetPrimaryPrice))
    (LocalVariables|SetText (Utilities|Text|FormatText "Hold F to buy {Name} [Cost: {Cost}]" (Variables|Default|GetItemName) (Variables|Default|GetCost)))
    (else
      (LocalVariables|SetText (Utilities|Text|FormatText "Hold F to Refill {Name} Ammo [Cost: {Cost}]" (Variables|Default|GetItemName) (Variables|Default|GetCost)))))
  (return (LocalVariables|GetText)))