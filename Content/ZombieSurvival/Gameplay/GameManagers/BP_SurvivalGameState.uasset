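; Game state Blueprint for the zombie survival mode that reacts to round, spawn-point and undead events, mostly with on-screen debug messages.
; Round changes announce the round number and undead count, while kills print the number left and spawns print the new undead's Health stat.
; AddRoundCounter creates a round counter widget for the player's controller and attaches it to that player's HUD border.
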(event Custom|Add%20Round%20Counter
  (params (Player :type BP%20Soldier%20Object%20Reference))
  (bind _asbp_player_controller (Utilities|Casting|CastToBP_PlayerController (Pawn|GetController Player)))
  (bind _returnvalue (UserInterface|CreateWidget "/Game/ZombieSurvival/UI/HUD/UI_Prefab_RoundCounter.UI_Prefab_RoundCounter_C" _asbp_player_controller))
  (bind _output_get (Variables|Default|SetRoundCounter _returnvalue))
  (Widget|Panel|AddChild (Variables|/Game/ZombieSurvival/UI/HUD/UI_MainHUD.UI_MainHUD_C|GetROundCounterBorder (Variables|/Game/ZombieSurvival/Characters/Blueprints/BP_Soldier.BP_Soldier_C|GetHUD Player)) _output_get))

(event Custom|ChangeRound
  (Development|PrintString (Utilities|String|ToString(Text) (Utilities|Text|FormatText "Round {Number} Has Begun! 
Undead This Round: {Amount}" (Variables|Default|GetRoundNumber) (Variables|Default|GetUndeadPerRound))) true true "(R=1.000000,G=0.750000,B=0.000000,A=1.000000)" 1e+01))

(event EventOnRoundChanged
  (params (UndeadAmount :type Integer))
  (CallFunction|ChangeRound))

(event EventOnUndeadKilled
  (Development|PrintString (Utilities|String|ToString(Text) (Utilities|Text|FormatText "{Amount} Undead Left" (Variables|Default|GetUndeadLeft)))))

(event EventOnSpawnLocationAdded
  (params (SpawnPoint :type Undead%20Spawn%20Point%20Object%20Reference))
  (Development|PrintString (Utilities|String|ToString(Text) (Utilities|Text|FormatText "{Name} has been Added to the List of Spawn Locations" (Utilities|GetDisplayName SpawnPoint)))))

(event EventOnUndeadSpawned
  (params (Undead :type Undead%20Object%20Reference))
  (bind _entitystatcomponent (Variables|/Script/Sample.Entity|GetEntityStatComponent Undead))
  (bind _returnvalue (Class|EntityStatComponent|FindStatAttribute _entitystatcomponent "Health"))
  (Development|PrintString (Utilities|String|ToString(Text) (Utilities|Text|FormatText "{Current} / {Total}" (Variables|/Script/Sample.StatAttribute|GetCurrentValue _returnvalue) (+ (Variables|/Script/Sample.StatAttribute|GetDefaultValue _returnvalue) (Variables|/Script/Sample.StatAttribute|GetBonusValue _returnvalue) (Variables|/Script/Sample.StatAttribute|GetInfiniteBonusValue _returnvalue))))))

(fn ConstructionScript)