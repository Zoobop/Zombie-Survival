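; BP_Undead_SpawnPoint is a spawn point that creates an undead actor at a random location within its box collision area.
; OnSpawnUndead calls ServerFindLocation, which prints a debug message and spawns the UndeadToSpawn class.
; The location is a random point in the box, built from the component's relative location and extent plus a fixed Z offset.
; Spawning adjusts for collisions where possible but always succeeds.
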(event Custom|Server%20Find%20Location
  (bind _boxcollision (Variables|Default|GetBoxCollision))
  (Development|PrintString "Server Spawned Undead")
  (Game|SpawnActorfromClass (Variables|Default|GetUndeadToSpawn) (Math|Conversions|ToTransform(Vector) (+ (Math|Random|RandomPointinBoundingBox (Variables|/Script/Engine.SceneComponent|GetRelativeLocation _boxcollision) (Variables|/Script/Engine.BoxComponent|GetBoxExtent _boxcollision)) "0, 0,94.000000")) "AdjustIfPossibleButAlwaysSpawn" 0 0))

(event EventOnSpawnUndead
  (CallFunction|ServerFindLocation))

(fn ConstructionScript)