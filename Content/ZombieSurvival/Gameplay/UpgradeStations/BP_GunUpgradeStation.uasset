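; Zombie survival station that sells an upgrade for the soldier's current weapon, prompting with the cost when the player lacks it.
; Trigger overlap toggles the prompt, player 0's input and a gate that lets Interact call Purchase.
; OnUpgrade adds the modifiers to the equipped weapon and reloads it, directly with authority or through Server calls otherwise.
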(event OnComponentBeginOverlap(PurchaseTrigger)
  (params (OverlappedComponent :type Primitive%20Component%20Object%20Reference) (OtherActor :type Actor%20Object%20Reference) (OtherComp :type Primitive%20Component%20Object%20Reference) (OtherBodyIndex :type Integer) (bFromSweep :type Boolean) (SweepResult :type Hit%20Result%20Structure%20%28by%20ref%29))
  (bind _asbp_soldier (Utilities|Casting|CastToBP_Soldier OtherActor))
  (Utilities|DisplayActionText _asbp_soldier)
  (Input|EnableInput (Game|GetPlayerController 0))
  (Utilities|FlowControl|Gate true) ; enters at Open
)

(event OnComponentEndOverlap(PurchaseTrigger)
  (params (OverlappedComponent :type Primitive%20Component%20Object%20Reference) (OtherActor :type Actor%20Object%20Reference) (OtherComp :type Primitive%20Component%20Object%20Reference) (OtherBodyIndex :type Integer))
  (bind _asbp_soldier (Utilities|Casting|CastToBP_Soldier OtherActor))
  (Utilities|RemoveDisplayText _asbp_soldier)
  (Input|DisableInput (Game|GetPlayerController 0))
  (Utilities|FlowControl|Gate true) ; enters at Close
)

(event EventOnUpgrade
  (params (Player :type Soldier%20Object%20Reference))
  (Utilities|AddUpgradeModifiers Player))

(event EventOnPostPurchase
  (Development|PrintString "Weapon has been upgraded" true true "(R=0.000854,G=1.000000,B=0.000000,A=1.000000)" 5.0))

(event Input|ActionEvents|InputActionInteract
  (params (Key :type Key%20Structure))
  (:Pressed
    (if (not (Class|UpgradeStation|HasUpgrade (stale OnComponentBeginOverlap(PurchaseTrigger) _asbp_soldier)))
      (Utilities|FlowControl|Gate true
        (:Exit
          (Class|GunUpgradeStation|Purchase (stale OnComponentBeginOverlap(PurchaseTrigger) _asbp_soldier))
          (Utilities|RemoveDisplayText (stale OnComponentBeginOverlap(PurchaseTrigger) _asbp_soldier)))))))

(fn ConstructionScript)