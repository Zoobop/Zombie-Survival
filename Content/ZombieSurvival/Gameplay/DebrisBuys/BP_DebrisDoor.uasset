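; BP_DebrisDoor is a buyable debris barrier for zombie survival that soldiers pay to clear.
; Its trigger shows a name-and-cost prompt and, on authority, registers the soldier and opens a gate that lets Activate call Purchase through MulticastPurchase.
; OnRemoveDebris sets HasBeenPurchased, whose RepNotify disables trigger and mesh collision, sinks the debris with a timeline, then hides it.
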(event OnComponentBeginOverlap(PurchaseTrigger)
  (params (OverlappedComponent :type Primitive%20Component%20Object%20Reference) (OtherActor :type Actor%20Object%20Reference) (OtherComp :type Primitive%20Component%20Object%20Reference) (OtherBodyIndex :type Integer) (bFromSweep :type Boolean) (SweepResult :type Hit%20Result%20Structure%20%28by%20ref%29))
  (bind (_asbp_soldier _bsuccess) (Utilities|Casting|CastToBP_Soldier OtherActor))
  (if _bsuccess
    (Default|DisplayActionText _asbp_soldier (Class|PurchasableInterface|GetDisplayText))
    (Networking|SwitchHasAuthority
      (:Authority
        (Default|InteractwithPurchaseable _asbp_soldier self true)
        (Input|EnableInput (Game|GetPlayerController 0))
        (Utilities|FlowControl|Gate true) ; enters at Open
      ))))

(event OnComponentEndOverlap(PurchaseTrigger)
  (params (OverlappedComponent :type Primitive%20Component%20Object%20Reference) (OtherActor :type Actor%20Object%20Reference) (OtherComp :type Primitive%20Component%20Object%20Reference) (OtherBodyIndex :type Integer))
  (bind (_asbp_soldier _bsuccess) (Utilities|Casting|CastToBP_Soldier OtherActor))
  (if _bsuccess
    (Default|RemoveActionText _asbp_soldier)
    (Networking|SwitchHasAuthority
      (:Authority
        (Default|InteractwithPurchaseable _asbp_soldier self false)
        (Input|DisableInput (Game|GetPlayerController 0))
        (Utilities|FlowControl|Gate true) ; enters at Close
      ))))

(event Custom|OnRepAction
  (bind _debrisbase (Variables|Default|GetDebrisBase))
  (Collision|SetCollisionResponsetoAllChannels (Variables|Default|GetPurchaseTrigger) "ECR_Ignore")
  (Collision|SetCollisionResponsetoAllChannels (Variables|Default|GetDebrisMesh) "ECR_Ignore")
  (Development|PrintString "Debris Removed")
  (Timeline|Door%20Slide Play
    (:Update
      (Transformation|AddWorldOffset _debrisbase "0, 0,-3.000000" false false))
    (:Finished
      (Development|SetHiddeninGame _debrisbase true true))))

(event Custom|Multicast%20Purchase
  (params (Player :type Soldier%20Object%20Reference))
  (Class|Debris|Purchase Player))

(event EventActivate
  (Utilities|FlowControl|Gate true
    (:Exit
      (CallFunction|MulticastPurchase (.AsBP%20Soldier (Utilities|Casting|CastToBP_Soldier (stale OnComponentBeginOverlap(PurchaseTrigger) OtherActor))))
      (Default|RemoveActionText (.AsBP%20Soldier (Utilities|Casting|CastToBP_Soldier (stale OnComponentBeginOverlap(PurchaseTrigger) OtherActor)))))))

(event EventOnRemoveDebris
  (params (Player :type Soldier%20Object%20Reference))
  (Variables|Default|SetHasBeenPurchased true))

(fn ConstructionScript)

(fn GetDisplayText
  (return (Utilities|Text|FormatText "Hold F to buy {Name} [Cost: {Cost}]" (Variables|Default|GetDebrisName) (Variables|Default|GetDebrisCost))))

(fn OnRepHasBeenPurchased
  (CallFunction|OnRepAction))