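; Purchasable perk station that grants Recovery Expert to a BP_Soldier in the zombie survival game.
; Overlapping the trigger shows a cost prompt for soldiers lacking the perk, enables player 0 input and opens a gate, closed again on exit.
; Pressing Interact through the gate calls Purchase.
; OnAcquirePerk applies PerkModifiers to the player's EntityStatComponent, broadcasts the stat change and adds the perk icon.
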(event OnComponentBeginOverlap(PurchaseTrigger)
  (params (OverlappedComponent :type Primitive%20Component%20Object%20Reference) (OtherActor :type Actor%20Object%20Reference) (OtherComp :type Primitive%20Component%20Object%20Reference) (OtherBodyIndex :type Integer) (bFromSweep :type Boolean) (SweepResult :type Hit%20Result%20Structure%20%28by%20ref%29))
  (bind _asbp_soldier (Utilities|Casting|CastToBP_Soldier OtherActor))
  (if (not (Class|PerkStation|HasPerk _asbp_soldier))
    (Default|DisplayActionText _asbp_soldier (Utilities|Text|FormatText "Hold F to buy {Name} [Cost: {Cost}]" (Variables|Default|GetPerkName) (Variables|Default|GetPerkCost)))
    (Input|EnableInput (Game|GetPlayerController 0))
    (Utilities|FlowControl|Gate true) ; enters at Open
  ))

(event OnComponentEndOverlap(PurchaseTrigger)
  (params (OverlappedComponent :type Primitive%20Component%20Object%20Reference) (OtherActor :type Actor%20Object%20Reference) (OtherComp :type Primitive%20Component%20Object%20Reference) (OtherBodyIndex :type Integer))
  (bind _asbp_soldier (Utilities|Casting|CastToBP_Soldier OtherActor))
  (Default|RemoveActionText _asbp_soldier)
  (Input|DisableInput 0)
  (Utilities|FlowControl|Gate true) ; enters at Close
)

(event EventOnPerkAcquisition)

(event EventOnAcquirePerk
  (params (Player :type Soldier%20Object%20Reference))
  (Class|RecoveryExpertPerkStation|RecoveryExpertPerk Player))

(event EventRecoveryExpertPerk
  (params (Player :type Soldier%20Object%20Reference))
  (bind _entitystatcomponent (Variables|/Script/Sample.Entity|GetEntityStatComponent Player))
  (Class|EntityStatComponent|ReceiveStatAttributeModification _entitystatcomponent (Variables|Default|GetPerkModifiers))
  (Default|CallOnStatAttributeChanged _entitystatcomponent)
  (bind _asbp_soldier (Utilities|Casting|CastToBP_Soldier Player))
  (Default|AddPerk _asbp_soldier (Variables|Default|GetPerkIcon)))

(event Input|ActionEvents|InputActionInteract
  (params (Key :type Key%20Structure))
  (:Pressed
    (if (not (Class|PerkStation|HasPerk (stale OnComponentBeginOverlap(PurchaseTrigger) _asbp_soldier)))
      (Utilities|FlowControl|Gate true
        (:Exit
          (Class|PerkStation|Purchase (stale OnComponentBeginOverlap(PurchaseTrigger) _asbp_soldier))
          (Default|RemoveActionText (stale OnComponentBeginOverlap(PurchaseTrigger) _asbp_soldier)))))))

(fn ConstructionScript)