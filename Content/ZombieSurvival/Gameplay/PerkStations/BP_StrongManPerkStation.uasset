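; Purchasable Strong Man perk station that boosts a soldier's stats through PerkModifiers in the zombie survival game.
; Trigger overlap shows a name-and-cost prompt to soldiers lacking the perk and, on authority, registers the purchasable, enables player-0 input and opens a gate.
; Activate purchases through that gate using the overlapped actor; leaving reverses the setup.
; Acquisition applies modifiers to EntityStatComponent, prints Health for debugging and adds the perk icon.
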(event OnComponentBeginOverlap(PurchaseTrigger)
  (params (OverlappedComponent :type Primitive%20Component%20Object%20Reference) (OtherActor :type Actor%20Object%20Reference) (OtherComp :type Primitive%20Component%20Object%20Reference) (OtherBodyIndex :type Integer) (bFromSweep :type Boolean) (SweepResult :type Hit%20Result%20Structure%20%28by%20ref%29))
  (bind (_asbp_soldier _bsuccess) (Utilities|Casting|CastToBP_Soldier OtherActor))
  (if _bsuccess
    (if (not (Class|PerkStation|HasPerk _asbp_soldier))
      (Default|DisplayActionText _asbp_soldier (Class|PurchasableInterface|GetDisplayText))
      (Networking|SwitchHasAuthority
        (:Authority
          (Default|InteractwithPurchaseable _asbp_soldier self true)
          (Input|EnableInput (Game|GetPlayerController 0))
          (Utilities|FlowControl|Gate true) ; enters at Open
        )))))

(event OnComponentEndOverlap(PurchaseTrigger)
  (params (OverlappedComponent :type Primitive%20Component%20Object%20Reference) (OtherActor :type Actor%20Object%20Reference) (OtherComp :type Primitive%20Component%20Object%20Reference) (OtherBodyIndex :type Integer))
  (bind (_asbp_soldier _bsuccess) (Utilities|Casting|CastToBP_Soldier OtherActor))
  (if _bsuccess
    (Default|RemoveActionText _asbp_soldier)
    (Networking|SwitchHasAuthority
      (:Authority
        (Default|InteractwithPurchaseable _asbp_soldier self false)
        (Input|DisableInput (Game|GetPlayerController 0))
        (Utilities|FlowControl|Gate true) ; enters at Close
      ))))

(event EventActivate
  (if (not (Class|PerkStation|HasPerk (.AsBP%20Soldier (Utilities|Casting|CastToBP_Soldier (stale OnComponentBeginOverlap(PurchaseTrigger) OtherActor)))))
    (Utilities|FlowControl|Gate true
      (:Exit
        (Class|PerkStation|Purchase (.AsBP%20Soldier (Utilities|Casting|CastToBP_Soldier (stale OnComponentBeginOverlap(PurchaseTrigger) OtherActor))))
        (Default|RemoveActionText (.AsBP%20Soldier (Utilities|Casting|CastToBP_Soldier (stale OnComponentBeginOverlap(PurchaseTrigger) OtherActor))))))))

(event EventOnAcquirePerk
  (params (Player :type Soldier%20Object%20Reference))
  (Class|StrongManPerkStation|StrongManPerk Player))

(event EventOnPerkAcquisition)

(event EventStrongManPerk
  (params (Player :type Soldier%20Object%20Reference))
  (bind _entitystatcomponent (Variables|/Script/Sample.Entity|GetEntityStatComponent Player))
  (bind _returnvalue (Class|EntityStatComponent|FindStatAttribute _entitystatcomponent "Health"))
  (Class|EntityStatComponent|ReceiveStatAttributeModification _entitystatcomponent (Variables|Default|GetPerkModifiers))
  (Default|CallOnStatAttributeChanged _entitystatcomponent)
  (Development|PrintString (Utilities|String|ToString(Text) (Utilities|Text|FormatText "Health: {Current} / {Total}" (Variables|/Script/Sample.StatAttribute|GetCurrentValue _returnvalue) (+ (Variables|/Script/Sample.StatAttribute|GetDefaultValue _returnvalue) (Variables|/Script/Sample.StatAttribute|GetBonusValue _returnvalue) (Variables|/Script/Sample.StatAttribute|GetInfiniteBonusValue _returnvalue)))) true true "(R=1.000000,G=0.016534,B=0.000000,A=1.000000)" 2e+01)
  (bind _asbp_soldier (Utilities|Casting|CastToBP_Soldier Player))
  (Default|AddPerk _asbp_soldier (Variables|Default|GetPerkIcon)))

(fn ConstructionScript)

(fn GetDisplayText
  (return (Utilities|Text|FormatText "Hold F to buy {Name} [Cost: {Cost}]" (Variables|Default|GetPerkName) (Variables|Default|GetPerkCost))))