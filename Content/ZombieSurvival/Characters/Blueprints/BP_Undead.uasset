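; BP_Undead is an undead character Blueprint that reacts to events from its EntityStatComponent.
; Stat attribute changes are printed on screen as debug text with tag, current and default values.
; On death it prints a message, plays a random soldier death montage, then destroys itself on a timer after the montage completes.
; The random range reaches only the first two of the three wired montages.
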(event OnStatAttributeChanged(EntityStatComponent)
  (params (StatAttribute :type Stat%20Attribute%20Object%20Reference))
  (Development|PrintString (Utilities|String|ToString(Text) (Utilities|Text|FormatText "{Name} : {Attribute Tag} [ {Current} / {Default}  ]" (Variables|/Script/Sample.EntityStatComponent|GetName (Variables|Default|GetEntityStatComponent)) (Variables|/Script/Sample.StatAttribute|GetStatAttributeTag StatAttribute) (Variables|/Script/Sample.StatAttribute|GetCurrentValue StatAttribute) (Variables|/Script/Sample.StatAttribute|GetDefaultValue StatAttribute))) true true "(R=0.000000,G=0.660000,B=1.000000,A=1.000000)" 1e+01))

(event OnHandleDeath(EntityStatComponent)
  (Development|PrintString "Entity is dead")
  (Animation|Montage|PlayMontage (Variables|Character|GetMesh) (Utilities|Select :Index (Math|Random|RandomInteger 2) :Option%200 "/Game/ZombieSurvival/Characters/Animations/AnimMontages/Soldier_Death_1.Soldier_Death_1" :Option%201 "/Game/ZombieSurvival/Characters/Animations/AnimMontages/Soldier_Death_2.Soldier_Death_2" :Option%202 "/Game/ZombieSurvival/Characters/Animations/AnimMontages/Soldier_Death_3.Soldier_Death_3")
    (:OnCompleted
      (Utilities|Time|SetTimerbyEvent (delegate Custom|Destroy) 5.0))))

(event Custom|Destroy
  (Actor|DestroyActor))

(fn ConstructionScript)