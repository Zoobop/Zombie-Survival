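; BP_Soldier is a soldier character Blueprint with weapon switching, aim-down-sights and crouch camera effects.
; Next and previous weapon inputs drive EquipmentComponent, whose equipment-changed and weapon-switched events refresh the displayed WeaponMesh.
; Reversible timelines animate FollowCamera's field of view for aiming and its relative height for crouching.
; EntityStatComponent attribute changes print to screen as debug text.
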(event OnWeaponSwitched(EquipmentComponent)
  (bind _returnvalue (Class|EquipmentComponent|DisplayWeaponMesh (Variables|Default|GetEquipmentComponent)))
  (Class|SkinnedMeshComponent|SetSkeletalMesh (Variables|Default|GetWeaponMesh) _returnvalue true))

(event OnEquipmentChanged(EquipmentComponent)
  (bind _returnvalue (Class|EquipmentComponent|DisplayWeaponMesh (Variables|Default|GetEquipmentComponent)))
  (Class|SkinnedMeshComponent|SetSkeletalMesh (Variables|Default|GetWeaponMesh) _returnvalue true))

(event OnStatAttributeChanged(EntityStatComponent)
  (params (StatAttribute :type Stat%20Attribute%20Object%20Reference))
  (Development|PrintString (Utilities|String|ToString(Text) (Utilities|Text|FormatText "{Name} : {Attribute Tag} [ {Current} / {Default}  ]" (Variables|/Script/Sample.EntityStatComponent|GetName (Variables|Default|GetEntityStatComponent)) (Variables|/Script/Sample.StatAttribute|GetStatAttributeTag StatAttribute) (Variables|/Script/Sample.StatAttribute|GetCurrentValue StatAttribute) (Variables|/Script/Sample.StatAttribute|GetDefaultValue StatAttribute))) true true "(R=0.000000,G=0.660000,B=1.000000,A=1.000000)" 1e+01))

(event EventOnStartADS
  ;[1 1 1] Aim Down Sights
  (bind _field_of_view (Timeline|Camera%20Zoom Play)
    (:Update
      (Camera|SetFieldOfView (Variables|Default|GetFollowCamera) _field_of_view))))

(event EventOnStopADS
  ;[1 1 1] Aim Down Sights
  (bind _field_of_view (Timeline|Camera%20Zoom Reverse)
    (:Update
      (Camera|SetFieldOfView (Variables|Default|GetFollowCamera) _field_of_view))))

(event EventOnStartCrouching
  (bind _followcamera (Variables|Default|GetFollowCamera))
  (bind _relativelocation (Variables|/Script/Engine.SceneComponent|GetRelativeLocation _followcamera))
  (bind _z (Timeline|Camera%20Drop Play)
    (:Update
      (Transformation|SetRelativeLocation _followcamera (Math|Vector|MakeVector (.x _relativelocation) (.y _relativelocation) _z) false false))))

(event EventOnStopCrouching
  (bind _followcamera (Variables|Default|GetFollowCamera))
  (bind _relativelocation (Variables|/Script/Engine.SceneComponent|GetRelativeLocation _followcamera))
  (bind _z (Timeline|Camera%20Drop Reverse)
    (:Update
      (Transformation|SetRelativeLocation _followcamera (Math|Vector|MakeVector (.x _relativelocation) (.y _relativelocation) _z) false false))))

(event Input|ActionEvents|InputActionJump
  (params (Key :type Key%20Structure :default "None"))
  ;[1 1 1] Input
)

(event Input|ActionEvents|InputActionProne
  (params (Key :type Key%20Structure :default "None"))
  ;[1 1 1] Input
)

(event Input|ActionEvents|InputActionNextWeapon
  (params (Key :type Key%20Structure :default "None"))
  ;[1 1 1] Switch Between Weapons
  (:Pressed
    (Class|EquipmentComponent|SwitchWeapon (Variables|Default|GetEquipmentComponent) 1)))

(event Input|ActionEvents|InputActionPreviousWeapon
  (params (Key :type Key%20Structure :default "None"))
  ;[1 1 1] Switch Between Weapons
  (:Pressed
    (Class|EquipmentComponent|SwitchWeapon (Variables|Default|GetEquipmentComponent) -1)))

(fn ConstructionScript)