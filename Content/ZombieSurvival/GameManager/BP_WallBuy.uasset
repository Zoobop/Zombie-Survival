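; BP_WallBuy is a wall-buy purchase point for the zombie survival mode, showing a buy prompt to a soldier in range.
; Overlapping PurchaseTrigger calls CheckItem on the BP_Soldier to choose the refill or first-purchase price, then shows the item name and cost on that soldier's HUD.
; Leaving the trigger hides and clears the prompt.
; OnRefill and OnFirstTimePurchase are empty events, and no purchase input or payment is handled here.
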(event OnComponentBeginOverlap(PurchaseTrigger)
  (params (OverlappedComponent :type Primitive%20Component%20Object%20Reference) (OtherActor :type Actor%20Object%20Reference) (OtherComp :type Primitive%20Component%20Object%20Reference) (OtherBodyIndex :type Integer) (bFromSweep :type Boolean) (SweepResult :type Hit%20Result%20Structure%20%28by%20ref%29))
  (bind _asbp_soldier (Utilities|Casting|CastToBP_Soldier OtherActor))
  (bind _returnvalue (Class|WallBuy|CheckItem _asbp_soldier))
  (if _returnvalue
    (Variables|Default|SetCost (Variables|Default|GetRefillPrice))
    (else
      (Variables|Default|SetCost (Variables|Default|GetPurchasePrice))))
  (Widget|SetVisibility (Variables|/Game/ZombieSurvival/UI/HUD/UI_MainHUD.UI_MainHUD_C|GetUI_Prefab_ActionText (Variables|/Game/ZombieSurvival/Characters/Blueprints/BP_Soldier.BP_Soldier_C|GetHUD _asbp_soldier)) "Visible")
  (Default|ChangeText (Variables|/Game/ZombieSurvival/UI/HUD/UI_MainHUD.UI_MainHUD_C|GetUI_Prefab_ActionText (Variables|/Game/ZombieSurvival/Characters/Blueprints/BP_Soldier.BP_Soldier_C|GetHUD _asbp_soldier)) (Utilities|Text|FormatText "Hold F to buy {Name} [Cost: {Cost}]" (Variables|Default|GetItemName) (Variables|Default|GetCost))))

(event OnComponentEndOverlap(PurchaseTrigger)
  (params (OverlappedComponent :type Primitive%20Component%20Object%20Reference) (OtherActor :type Actor%20Object%20Reference) (OtherComp :type Primitive%20Component%20Object%20Reference) (OtherBodyIndex :type Integer))
  (bind _asbp_soldier (Utilities|Casting|CastToBP_Soldier OtherActor))
  (Widget|SetVisibility (Variables|/Game/ZombieSurvival/UI/HUD/UI_MainHUD.UI_MainHUD_C|GetUI_Prefab_ActionText (Variables|/Game/ZombieSurvival/Characters/Blueprints/BP_Soldier.BP_Soldier_C|GetHUD _asbp_soldier)) "Hidden")
  (Default|ChangeText (Variables|/Game/ZombieSurvival/UI/HUD/UI_MainHUD.UI_MainHUD_C|GetUI_Prefab_ActionText (Variables|/Game/ZombieSurvival/Characters/Blueprints/BP_Soldier.BP_Soldier_C|GetHUD _asbp_soldier))))

(event EventOnRefill
  (params (Player :type Soldier%20Object%20Reference)))

(event EventOnFirstTimePurchase
  (params (Player :type Soldier%20Object%20Reference)))

(fn ConstructionScript)