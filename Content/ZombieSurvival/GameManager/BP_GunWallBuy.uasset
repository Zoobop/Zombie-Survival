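; Wall-buy station in a zombie survival game that sells a gun, or an ammo refill at a secondary price.
; Overlapping soldiers see a cost prompt and open a gate letting Interact call Purchase.
; Purchase handlers add the gun or reload the matching equipped weapon, then deduct player-state points.
; Without authority, handlers run locally alongside a server event call; with authority, they run directly.
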(event OnComponentBeginOverlap(PurchaseTrigger)
  (params (OverlappedComponent :type Primitive%20Component%20Object%20Reference) (OtherActor :type Actor%20Object%20Reference) (OtherComp :type Primitive%20Component%20Object%20Reference) (OtherBodyIndex :type Integer) (bFromSweep :type Boolean) (SweepResult :type Hit%20Result%20Structure%20%28by%20ref%29))
  (bind _asbp_soldier (Utilities|Casting|CastToBP_Soldier OtherActor))
  (|DisplayText _asbp_soldier)
  (Input|EnableInput (Game|GetPlayerController 0))
  (Utilities|FlowControl|Gate true) ; enters at Open
)

(event OnComponentEndOverlap(PurchaseTrigger)
  (params (OverlappedComponent :type Primitive%20Component%20Object%20Reference) (OtherActor :type Actor%20Object%20Reference) (OtherComp :type Primitive%20Component%20Object%20Reference) (OtherBodyIndex :type Integer))
  (bind _asbp_soldier (Utilities|Casting|CastToBP_Soldier OtherActor))
  (|RemoveDisplay _asbp_soldier)
  (Input|DisableInput (Game|GetPlayerController 0))
  (Utilities|FlowControl|Gate true) ; enters at Close
)

(event Custom|Server%20On%20Refill
  (params (Player :type Soldier%20Object%20Reference))
  (Utilities|HandleRefill Player))

(event Custom|Server%20On%20First%20Time%20Purchase
  (params (Player :type Soldier%20Object%20Reference))
  (Utilities|HandleFirstTimePurchase Player))

(event EventOnFirstTimePurchase
  (params (Player :type Soldier%20Object%20Reference))
  (if (Ability|HasAuthority Player)
    (Utilities|HandleFirstTimePurchase Player)
    (else
      (CallFunction|ServeronFirstTimePurchase Player)
      (Utilities|HandleFirstTimePurchase Player))))

(event EventOnRefill
  (params (Player :type Soldier%20Object%20Reference))
  (if (Ability|HasAuthority Player)
    (Utilities|HandleRefill Player)
    (Development|PrintString "Server")
    (else
      (CallFunction|ServeronRefill Player)
      (Utilities|HandleRefill Player)
      (Development|PrintString "Client"))))

(event Input|ActionEvents|InputActionInteract
  (params (Key :type Key%20Structure))
  (:Pressed
    (Utilities|FlowControl|Gate true
      (:Exit
        (Class|WallBuy|Purchase (stale OnComponentBeginOverlap(PurchaseTrigger) _asbp_soldier))))))

(fn ConstructionScript)