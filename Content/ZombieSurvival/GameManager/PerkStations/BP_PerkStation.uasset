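; BP_PerkStation is a zombie survival station where a soldier buys a perk that modifies their stats.
; Overlapping the purchase trigger shows a name-and-cost prompt for unowned perks, enables input for player 0 and opens a Gate.
; Pressing Interact while the gate is open calls Purchase and clears the prompt.
; OnAcquirePerk applies the perk modifiers through the player's EntityStatComponent and prints the resulting Health.
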(event OnComponentBeginOverlap(PurchaseTrigger)
  (params (OverlappedComponent :type Primitive%20Component%20Object%20Reference) (OtherActor :type Actor%20Object%20Reference) (OtherComp :type Primitive%20Component%20Object%20Reference) (OtherBodyIndex :type Integer) (bFromSweep :type Boolean) (SweepResult :type Hit%20Result%20Structure%20%28by%20ref%29))
  (bind _asbp_soldier (Utilities|Casting|CastToBP_Soldier OtherActor))
  (Utilities|DisplayActionText _asbp_soldier)
  (Input|EnableInput (Game|GetPlayerController 0))
  (Utilities|FlowControl|Gate true) ; enters at Open
)

(event OnComponentEndOverlap(PurchaseTrigger)
  (params (OverlappedComponent :type Primitive%20Component%20Object%20Reference) (OtherActor :type Actor%20Object%20Reference) (OtherComp :type Primitive%20Component%20Object%20Reference) (OtherBodyIndex :type Integer))
  (bind _asbp_soldier (Utilities|Casting|CastToBP_Soldier OtherActor))
  (Utilities|RemoveDisplayText _asbp_soldier)
  (Input|DisableInput (Game|GetPlayerController 0))
  (Utilities|FlowControl|Gate true) ; enters at Close
)

(event EventOnAcquirePerk
  (params (Player :type Soldier%20Object%20Reference))
  (bind _entitystatcomponent (Variables|/Script/Sample.Entity|GetEntityStatComponent Player))
  (bind _returnvalue (Class|EntityStatComponent|FindStatAttribute _entitystatcomponent "Health"))
  (Class|EntityStatComponent|ReceiveStatAttributeModification _entitystatcomponent (Variables|Default|GetPerkModifiers))
  (Default|CallOnStatAttributeChanged _entitystatcomponent)
  (Development|PrintString (Utilities|String|ToString(Text) (Utilities|Text|FormatText "Health: {Current} / {Total}" (Variables|/Script/Sample.StatAttribute|GetCurrentValue _returnvalue) (+ (Variables|/Script/Sample.StatAttribute|GetDefaultValue _returnvalue) (Variables|/Script/Sample.StatAttribute|GetBonusValue _returnvalue) (Variables|/Script/Sample.StatAttribute|GetInfiniteBonusValue _returnvalue)))) true true "(R=1.000000,G=0.016534,B=0.000000,A=1.000000)" 2e+01))

(event Input|ActionEvents|InputActionInteract
  (params (Key :type Key%20Structure :default "None"))
  (:Pressed
    (if (not (Class|PerkStation|HasPerk (stale OnComponentBeginOverlap(PurchaseTrigger) _asbp_soldier)))
      (Utilities|FlowControl|Gate true
        (:Exit
          (Class|PerkStation|Purchase (stale OnComponentBeginOverlap(PurchaseTrigger) _asbp_soldier))
          (Utilities|RemoveDisplayText (stale OnComponentBeginOverlap(PurchaseTrigger) _asbp_soldier)))))))

(fn ConstructionScript)